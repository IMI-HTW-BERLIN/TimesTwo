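; Rotating laser hazard actor with two beams that damage the FirstPersonCharacter on contact.
; Each Tick it spins the root in yaw by TimeDilation times RotationSpeed, unscaled by delta time, and handles both beams.
; Each beam line-traces on Visibility towards forward vector times MaxDistance, without adding its location.
; A hit moves the beam's target to the impact point and, on the character, applies LaserDamage every frame, printing the result.
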(event EventTick
  (params (DeltaSeconds :type Float%20%28single-precision%29))
  (CallFunction|HandleLaser (Variables|Default|GetBeam1))
  (CallFunction|HandleLaser (Variables|Default|GetBeam2))
  (Transformation|AddWorldRotation (Variables|Default|GetDefaultSceneRoot) (Math|Rotator|MakeRotator 0.0 0.0 (* (Variables|Default|GettimeDilation) (Variables|Default|GetrotationSpeed))) false false))

(fn ConstructionScript)

(fn SetLaserTarget
  (params (beam :type Particle%20System%20Component%20Object%20Reference))
  (bind (_outhit _returnvalue) (Collision|LineTraceByChannel (Transformation|GetWorldLocation beam) (* (Math|Vector|GetForwardVector beam) (Variables|Default|GetmaxDistance)) "TraceTypeQuery1" false 0 "None"))
  (if _returnvalue
    (Class|ParticleSystemComponent|SetBeamTargetPoint beam 0 (.ImpactPoint (Collision|BreakHitResult _outhit)))
    (return (.HitActor (Collision|BreakHitResult _outhit)))))

(fn HandleLaser
  (params (beam :type Particle%20System%20Component%20Object%20Reference))
  (bind _hitactor (CallFunction|SetLaserTarget beam))
  (bind _asfirst_person_character (Utilities|Casting|CastToFirstPersonCharacter _hitactor))
  (bind _returnvalue (Game|Damage|ApplyDamage _asfirst_person_character (Variables|Default|GetlaserDamage) 0 self))
  (Development|PrintString (Utilities|String|ToString(Float) _returnvalue)))