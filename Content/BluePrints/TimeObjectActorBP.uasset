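; TimeObjectActorBP is a physics actor with its own time dilation, letting its motion be slowed or sped up.
; Tick applies a custom Gravity acceleration, while BeforeTick lerps linear and angular velocities from their last stored values toward current physics values, weighted by TimeDilation.
; SetTimeDilation rescales both velocities and Gravity by the new-to-old dilation ratio, overwriting the stored velocities.
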(event EventTick
  (params (DeltaSeconds :type Float%20%28single-precision%29))
  ;[1 1 1] Artificial gravity for custom gravity
  (Physics|AddForce (Variables|Default|GetPrimitiveType) (Variables|Default|GetGravity) "None" true))

(event EventBeforeTick
  (CallFunction|SetAngularVelocity)
  (CallFunction|SetLinearVelocity))

(event EventBeginPlay
  ;[1 1 1] Set start values
  (bind _output_get (Variables|Default|SetPrimitiveComp (Actor|GetComponentbyClass "/Script/Engine.PrimitiveComponent")))
  (Variables|Default|SetLastPosition (Transformation|GetActorLocation))
  (bind _returnvalue (Physics|GetPhysicsLinearVelocity _output_get "None"))
  (Variables|Default|SetLastLinearVelocity _returnvalue)
  (Variables|Default|SetLastAngularVelocity (Physics|GetPhysicsAngularVelocityinDegrees _output_get "None")))

(fn ConstructionScript)

(fn GetVectorBetween
  (params (FirstVector :type Vector) (SecondVector :type Vector) (Weight :type Float%20%28single-precision%29))
  (return (Math|Vector|Lerp(Vector) FirstVector SecondVector Weight)))

(fn SetAngularVelocity
  (bind _newvector (CallFunction|GetVectorBetween (Variables|Default|GetLastAngularVelocity) (Physics|GetPhysicsAngularVelocityinDegrees (Variables|Default|GetPrimitiveComp) "None") (Variables|Default|GetTimeDilation)))
  (bind _output_get (Variables|Default|SetLastAngularVelocity _newvector))
  (Class|PrimitiveComponent|SetPhysicsAngularVelocityinDegrees (Variables|Default|GetPrimitiveComp) _output_get false "None")
  (return _output_get))

(fn SetLinearVelocity
  (bind _returnvalue (Physics|GetPhysicsLinearVelocity (Variables|Default|GetPrimitiveComp) "None"))
  (bind _newvector (CallFunction|GetVectorBetween (Variables|Default|GetLastLinearVelocity) _returnvalue (Variables|Default|GetTimeDilation)))
  (bind _output_get (Variables|Default|SetLastLinearVelocity _newvector))
  (Physics|SetPhysicsLinearVelocity (Variables|Default|GetPrimitiveComp) _output_get false "None")
  (return _output_get))

(fn OverwriteLinearVelocity
  (params (NewVelocity :type Vector))
  (bind _output_get (Variables|Default|SetLastLinearVelocity NewVelocity))
  (Physics|SetPhysicsLinearVelocity (Variables|Default|GetPrimitiveType) _output_get false "None"))

(fn SetTimeDilation
  (params (NewTimeDilation :type Float%20%28single-precision%29))
  (bind _returnvalue (Physics|GetPhysicsLinearVelocity (Variables|Default|GetPrimitiveType) "None"))
  (CallFunction|OverwriteLinearVelocity (* _returnvalue (/ NewTimeDilation (Variables|Default|GetTimeDilation))))
  (CallFunction|OverwriteAngularVelocity (* (Physics|GetPhysicsAngularVelocityinDegrees (Variables|Default|GetPrimitiveType) "None") (/ NewTimeDilation (Variables|Default|GetTimeDilation))))
  (Variables|Default|SetGravity (* (Variables|Default|GetGravity) (/ NewTimeDilation (Variables|Default|GetTimeDilation))))
  (Variables|Default|SetTimeDilation NewTimeDilation))

(fn OverwriteAngularVelocity
  (params (NewAngularVelocity :type Vector))
  (bind _output_get (Variables|Default|SetLastAngularVelocity NewAngularVelocity))
  (Class|PrimitiveComponent|SetPhysicsAngularVelocityinDegrees (Variables|Default|GetPrimitiveType) _output_get false "None"))