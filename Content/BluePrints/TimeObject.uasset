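; TimeObject is an actor that shows a particle effect while its time dilation is below normal.
; SetTimeDilation stores the new value, and Tick checks it every frame to activate the particle system below 1.0 or deactivate it otherwise.
; The construction script passes the actor itself as the particle system's VertSurfaceActor parameter.
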(event EventTick
  (params (DeltaSeconds :type Float%20%28single-precision%29))
  (if (>= (Variables|Default|GettimeDilation) 1.0)
    (Components|Activation|Deactivate (Variables|Default|GetParticleSystem))
    (else
      (Components|Activation|Activate (Variables|Default|GetParticleSystem) false))))

(fn ConstructionScript
  (Effects|Components|ParticleSystem|SetActorParameter (Variables|Default|GetParticleSystem) "VertSurfaceActor" self))

(fn SetTimeDilation
  (params (newDilation :type Float%20%28single-precision%29))
  (Variables|Default|SettimeDilation newDilation))