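; Physics variant of a time-dilatable base actor that slows or speeds its physics body according to its own TimeDilation.
; Each tick it blends last and current linear and angular velocity by TimeDilation, scaling velocity changes, then applies a custom Gravity acceleration.
; SetTimeDilation rescales both velocities and Gravity by the new-to-old ratio before calling the parent.
; Overwrite functions set velocity and its cached value together, bypassing the blend.
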(event EventTick
  (params (DeltaSeconds :type Float%20%28single-precision%29))
  (bind _primitivetype (Variables|Default|GetPrimitiveType))
  (|CallParentFunction DeltaSeconds)
  ;[1 1 1] Set Velocity
  (CallFunction|SetAngularVelocity _primitivetype)
  (CallFunction|SetLinearVelocity _primitivetype)
  ;[1 1 1] Artificial gravity for custom gravity
  (Physics|AddForce (Variables|Default|GetPrimitiveType) (Variables|Default|Getgravity) "None" true))

(event EventBeginPlay
  (bind _primitivetype (Variables|Default|GetPrimitiveType))
  (|CallParentFunction)
  ;[1 1 1] Set start values
  (Variables|Default|SetlastPosition (Transformation|GetActorLocation))
  (bind _returnvalue (Physics|GetPhysicsLinearVelocity _primitivetype "None"))
  (Variables|Default|SetlastLinearVelocity _returnvalue)
  (Variables|Default|SetlastAngularVelocity (Physics|GetPhysicsAngularVelocityinDegrees _primitivetype "None")))

(fn ConstructionScript
  (|CallParentFunction))

(fn GetVectorBetween
  (params (FirstVector :type Vector) (SecondVector :type Vector) (Weight :type Float%20%28single-precision%29))
  (return (+ FirstVector (* (- SecondVector FirstVector) Weight))))

(fn SetAngularVelocity
  (params (physicsObject :type Primitive%20Component%20Object%20Reference%20%28by%20ref%29))
  (bind _newvector (CallFunction|GetVectorBetween (Variables|Default|GetlastAngularVelocity) (Physics|GetPhysicsAngularVelocityinDegrees physicsObject "None") (Variables|Default|GettimeDilation)))
  (bind _output_get (Variables|Default|SetlastAngularVelocity _newvector))
  (Class|PrimitiveComponent|SetPhysicsAngularVelocityinDegrees physicsObject _output_get false "None")
  (return _output_get))

(fn SetLinearVelocity
  (params (physicsObject :type Primitive%20Component%20Object%20Reference%20%28by%20ref%29))
  (bind _returnvalue (Physics|GetPhysicsLinearVelocity physicsObject "None"))
  (bind _newvector (CallFunction|GetVectorBetween (Variables|Default|GetlastLinearVelocity) _returnvalue (Variables|Default|GettimeDilation)))
  (bind _output_get (Variables|Default|SetlastLinearVelocity _newvector))
  (Physics|SetPhysicsLinearVelocity physicsObject _output_get false "None")
  (return _output_get))

(fn OverwriteLinearVelocity
  (params (NewVelocity :type Vector))
  (bind _output_get (Variables|Default|SetlastLinearVelocity NewVelocity))
  (Physics|SetPhysicsLinearVelocity (Variables|Default|GetPrimitiveType) _output_get false "None"))

(fn OverwriteAngularVelocity
  (params (NewAngularVelocity :type Vector))
  (bind _output_get (Variables|Default|SetlastAngularVelocity NewAngularVelocity))
  (Class|PrimitiveComponent|SetPhysicsAngularVelocityinDegrees (Variables|Default|GetPrimitiveType) _output_get false "None"))

(fn SetTimeDilation
  (params (newDilation :type Float%20%28single-precision%29))
  (bind _timedilation (Variables|Default|GettimeDilation))
  (bind _returnvalue (/ newDilation _timedilation))
  (bind _returnvalue_2 (Physics|GetPhysicsLinearVelocity (Variables|Default|GetPrimitiveType) "None"))
  (CallFunction|OverwriteLinearVelocity (* _returnvalue_2 _returnvalue))
  (CallFunction|OverwriteAngularVelocity (* (Physics|GetPhysicsAngularVelocityinDegrees (Variables|Default|GetPrimitiveType) "None") _returnvalue))
  (Variables|Default|Setgravity (* (Variables|Default|Getgravity) _returnvalue))
  (|CallParentFunction newDilation))