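; Base Activator Blueprint that triggers a linked Activatable when interacted with.
; Interact sets IsActivated, then calls Activate on the Activatable, but only if any linked SiblingActivator is also activated, allowing paired activators.
; With KeepActivating set, Tick accumulates a timer and calls Interact again each time it reaches ActivationTimer.
; IsActivated is never cleared here.
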(event EventTick
  (params (DeltaSeconds :type Float%20%28single-precision%29))
  (if (and (Variables|Default|GetisActivated) (Variables|Default|GetkeepActivating))
    (if (>= (Variables|Default|Gettimer) (Variables|Default|GetactivationTimer))
      (Variables|Default|Settimer 0.0)
      (CallFunction|Interact)
      (else
        (Variables|Default|Settimer (+ (Variables|Default|Gettimer) DeltaSeconds))))))

(fn ConstructionScript)

(fn Interact
  (bind _activatable (Variables|Default|GetActivatable))
  (Variables|Default|SetisActivated true)
  (if (Utilities|IsValid (Variables|Default|GetSiblingActivator))
    (if (Variables|Activator_C|GetisActivated (Variables|Default|GetSiblingActivator))
      (if (Utilities|IsValid _activatable) :!label _label
        (Default|Activate _activatable)))
    (else
      (goto _label))))