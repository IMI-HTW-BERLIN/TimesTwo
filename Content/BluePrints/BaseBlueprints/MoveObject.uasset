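; MoveObject is a base Blueprint for moving a primitive component along a looping list of patrol points, though the movement is unfinished.
; Tick gets a normalized direction toward the current point, but applies a zero relative offset without sweep.
; The direction, MovementSpeed and delta time product is left unconnected.
; SelectNextPatrolPoint advances the index with wraparound, but nothing in these graphs calls it.
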(event EventTick
  (params (DeltaSeconds :type Float%20%28single-precision%29))
  (|CallParentFunction DeltaSeconds)
  (bind _direction (CallFunction|GetMovementDirection))
  (if true
    (Transformation|AddRelativeLocation (Variables|Default|GetPrimitiveType) "0, 0, 0" false false)))

(fn ConstructionScript
  (|CallParentFunction))

(fn SelectNextPatrolPoint
  (Variables|Default|SetcurrentPatrolPoint (Math|Integer|%(Integer) (+ (Variables|Default|GetcurrentPatrolPoint) 1) (Utilities|Array|Length (Variables|Default|GetpatrolPoints)))))

(fn GetMovementDirection
  (return (Math|Vector|Normalize (- (Utilities|Array|Get(acopy) (Variables|Default|GetpatrolPoints) (Variables|Default|GetcurrentPatrolPoint)) (Variables|/Script/Engine.SceneComponent|GetRelativeLocation (Variables|Default|GetPrimitiveType))))))